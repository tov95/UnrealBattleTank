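; AutoMortar_BP is an automated mortar enemy, a tank-style unit with a turret, barrel and health bar.
; On BeginPlay it hands the mortar barrel and turret to its TankAiming component and links itself to the HealthBar_BP widget shown on its widget component.
; When unpossessed, it activates the DeathBlast effect.
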(event `self.ReceiveUnpossessed`
  (params (OldController :type "Controller Object Reference"))
  (if true
    (`ActorComponent.Activate` (`self.DeathBlast`) false)))

(event `self.ReceiveBeginPlay`
  (`TankAimingComponent.Initialise` (`self.TankAiming`) (`self.MortarBarrel`) (`self.MortarTurret`))
  (`self.InitialiseHealthBarWidget`))

(fn `InitialiseHealthBarWidget`
  (bind _ashealth_bar_bp (cast `/Game/UI/HealthBar_BP` (`WidgetComponent.GetUserWidgetObject` (`self.HealthBarWidget`))))
  (set `/Game/UI/HealthBar_BP.Tank` self _ashealth_bar_bp))

(fn `UserConstructionScript`)